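; Rotating bridge actor that pitches into place once the player has collected the required number of points.
; A looping one-second timer checks CharacterBP's Points against PointsReq and plays the BridgeRotate timeline only on an exact match, stopping it otherwise.
; Each timeline update adds the animated pitch to the rotation captured at BeginPlay.
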(event `self.ReceiveBeginPlay`
  (`KismetSystemLibrary.K2_SetTimerDelegate` (delegate `CheckPlayerPoints`) 1.0 true)
  (bind _output_get (set `self.InitialRotation` (`self.K2_GetActorRotation`))))

(event `CheckPlayerPoints`
  (bind _ascharacter_bp (cast `/Game/Blueprint/BP_Char/CharacterBP` (`GameplayStatics.GetPlayerPawn` 0)))
  (if (== (`/Game/Blueprint/BP_Char/CharacterBP.Points` _ascharacter_bp) (`self.PointsReq`))
    (bind (_direction _bridgerotation) (`Timeline|BridgeRotate` :!label _label)
      (:`Update`
        (`self.K2_SetActorRotation` (`KismetMathLibrary.ComposeRotators` (stale `self.ReceiveBeginPlay` _output_get) (`KismetMathLibrary.MakeRotator` 0.0 _bridgerotation)))))
    (else
      (goto _label :!via `Stop`))))

(fn `UserConstructionScript`)
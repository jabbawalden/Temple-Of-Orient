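; Sphere obstacle that kills the player character on contact and recycles itself after falling out.
; Overlapping a FallKillVolume_Blueprint teleports the mesh to a hardcoded world location and zeroes its linear velocity.
; A hit on a CharacterBP calls Death, then a retriggerable delay leads to Respawn on player 0's pawn.
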(event `self.StaticMesh.OnComponentBeginOverlap`
  (params (OverlappedComponent :type "PrimitiveComponent Object Reference") (OtherActor :type "Actor Object Reference") (OtherComp :type "PrimitiveComponent Object Reference") (OtherBodyIndex :type Integer) (bFromSweep :type Boolean) (SweepResult :type "HitResult Structure (by ref)"))
  ;[1 1 1] Respawn
  (cast `/Game/Blueprint/FallKillVolume_Blueprint` OtherActor)
  (`SceneComponent.K2_SetWorldLocationAndRotation` :`self` (`self.StaticMesh`) :`NewLocation` (-120230.0 -138660.0 740360.0))
  (`PrimitiveComponent.SetPhysicsLinearVelocity` (`self.StaticMesh`) (0.0 0.0 0.0) false "None"))

(event `self.StaticMesh.OnComponentHit`
  (params (HitComponent :type "PrimitiveComponent Object Reference") (OtherActor :type "Actor Object Reference") (OtherComp :type "PrimitiveComponent Object Reference") (NormalImpulse :type "Vector Structure") (Hit :type "HitResult Structure (by ref)"))
  ;[1 1 1] KillPlayer
  (bind _ascharacter_bp (cast `/Game/Blueprint/BP_Char/CharacterBP` OtherActor))
  (`/Game/Blueprint/BP_Char/CharacterBP.Death` _ascharacter_bp)
  (`KismetSystemLibrary.RetriggerableDelay` 2.0)
  (bind _ascharacter_bp_2 (cast `/Game/Blueprint/BP_Char/CharacterBP` (`GameplayStatics.GetPlayerPawn` 0)))
  (`/Game/Blueprint/BP_Char/CharacterBP.Respawn` _ascharacter_bp_2))

(fn `UserConstructionScript`)
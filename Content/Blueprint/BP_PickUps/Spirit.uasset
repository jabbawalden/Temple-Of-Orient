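; Spirit pickup actor that spins and bobs in the world and destroys itself when player pawn 0 overlaps it, with no other effect.
; A timeline started on BeginPlay sets yaw on top of InitialRotation, though the node that captures that rotation is unconnected.
; A Bob timeline, told to Play every Tick, adds its ZAction output as a local offset on each update.
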(event EventBeginPlay
  (bind _rotate (Timeline|Timeline_0 Play)
    (:Update
      (Transformation|SetActorRotation (Math|Rotator|CombineRotators (stale _output_get) (Math|Rotator|MakeRotator 0.0 0.0 _rotate))))))

(event Collision|EventActorBeginOverlap
  (params (OtherActor :type Actor%20Object%20Reference))
  (if (== OtherActor (Game|Player|GetPlayerPawn 0))
    (Actor|DestroyActor)))

(event EventTick
  (params (DeltaSeconds :type Float%20%28single-precision%29))
  (bind _z_action (Timeline|Bob Play)
    (:Update
      (Transformation|AddActorLocalOffset _z_action false false))))

(fn ConstructionScript)